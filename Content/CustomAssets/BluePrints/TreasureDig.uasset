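; TreasureDig is a dig-spot actor that lets the player dig up an item.
; Overlap by a ThirdPersonCharacter toggles its input, so the 1 key works only within range.
; Pressing it loops the Digging animation for a ten-second delay, then restores the animation blueprint.
; It then sets CurrentItemId, adds ItemData to its own Inventory, leaving the character's Inventory unused, and prints the find.
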(event Collision|EventActorBeginOverlap
  (params (OtherActor :type Actor%20Object%20Reference))
  (bind _asthird_person_character (Utilities|Casting|CastToThirdPersonCharacter OtherActor))
  (Input|EnableInput (Game|GetPlayerController 0)))

(event Collision|EventActorEndOverlap
  (params (OtherActor :type Actor%20Object%20Reference))
  (Utilities|Casting|CastToThirdPersonCharacter OtherActor)
  (Input|DisableInput (Game|GetPlayerController 0)))

(event Input|KeyboardEvents|1
  (params (Key :type Key%20Structure))
  (bind _itemdata (Variables|Default|GetItemData))
  (bind (_name _thumbnail _description _isconsumable _itemid _weight _itemclass _istool _isfood _isdrink) (Utilities|Struct|BreakItemDataStructure _itemdata))
  (:Pressed
    (bind _asthird_person_character (Utilities|Casting|CastToThirdPersonCharacter (stale Collision|EventActorBeginOverlap _asthird_person_character)))
    (Components|Animation|PlayAnimation (Variables|/Script/Engine.Character|GetMesh _asthird_person_character) "/Game/Digging.Digging" true)
    (Utilities|FlowControl|Delay 1e+01)
    (Components|Animation|SetAnimationMode (Variables|/Script/Engine.Character|GetMesh _asthird_person_character) "AnimationBlueprint")
    (bind _asthird_person_character_2 (Utilities|Casting|CastToThirdPersonCharacter (Game|GetPlayerCharacter 0)))
    (Variables|Default|SetCurrentItemId 235.0)
    (Utilities|Array|Add (Variables|Default|GetInventory) (Utilities|Struct|MakeItemDataStructure _name _thumbnail _description _isconsumable _itemid _weight _itemclass _istool _isfood _isdrink))
    (Development|PrintString (Utilities|String|Append "you have found a" _name))))

(fn ConstructionScript)